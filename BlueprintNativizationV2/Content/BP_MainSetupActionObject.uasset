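; BP_MainSetupActionObject is an editor action object that launches the EU_NativizationTool utility widget to generate code for a single Blueprint node.
; ActionToNode opens the widget, sets it to one-function mode with the given Blueprint, selects the node name, hides header code, shows it fullscreen and runs code generation.
; ActionToProeprty is an empty stub taking a property name.
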(fn `ActionToNode`
  (params (ActionName :type Name) (NodeName :type Name) (Blueprint :type "Blueprint Object Reference"))
  (locals (NativizationTool :type "/BlueprintNativizationV2/EU_NativizationTool Object Reference"))
  (bind _returnvalue (`BlueprintNativizationLibrary.OpenEditorUtilityWidget` (`self.Widget Blueprint`)))
  (bind _aseu_nativization_tool (cast `/BlueprintNativizationV2/EU_NativizationTool` _returnvalue))
  (set `local.NativizationTool` _aseu_nativization_tool)
  (set `/BlueprintNativizationV2/EU_NativizationTool.GenerateCodeOneFunction` true (`local.NativizationTool`))
  (set `/BlueprintNativizationV2/EU_NativizationTool.Blueprints` (make `BlueprintProxy` (`|MakeArray` (`local.Blueprint`))) (`local.NativizationTool`))
  (`/BlueprintNativizationV2/EU_NativizationTool.UpdateFunctionNameDisableImage` (`local.NativizationTool`))
  (`/BlueprintNativizationV2/EU_NativizationTool.Initialization` (`local.NativizationTool`))
  (`ComboBoxString.SetSelectedOption` (`/BlueprintNativizationV2/EU_NativizationTool.FunctionNameSelect` (`local.NativizationTool`)) (`KismetStringLibrary.Conv_NameToString` (`local.NodeName`)))
  (set `/BlueprintNativizationV2/EU_NativizationTool.Show H Code` false (`local.NativizationTool`))
  (`ScrollBox.ScrollToEnd` (`/BlueprintNativizationV2/EU_NativizationTool.EditorUtilityScrollBox` (`local.NativizationTool`)))
  (`BlueprintNativizationLibrary.OpenWidgetToFullscreen` (`local.NativizationTool`))
  (`/BlueprintNativizationV2/EU_NativizationTool.ApplyCodeGeneration` (`local.NativizationTool`)))

(fn `ActionToProeprty`
  (params (ActionName :type Name) (PropertyName :type Name) (Blueprint :type "Blueprint Object Reference"))
  (locals (NativizationTool :type "/BlueprintNativizationV2/EU_NativizationTool Object Reference")))